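; Player-controlled flying ship pawn that thrusts, pitches, rolls and fires projectiles from twin guns.
; Thrust adds forward velocity to the physics BodyMesh, and pitch input also nudges velocity along that axis.
; Pitch and roll combine added angular velocity with direct local rotation, with roll adding slight yaw.
; Fire spawns a projectile at each rotated gun offset, but plays sounds at the untransformed offsets.
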(event Input|ActionEvents|InputActionFire
  (bind _returnvalue (Transformation|GetActorRotation))
  (bind _leftgunloc (Variables|Default|GetLeftGunLoc))
  ;[1 1 1] Fire Guns
  (:Pressed
    (Game|SpawnActorfromClass "/Game/Blueprints/Projectile.Projectile_C" (Math|Transform|MakeTransform (+ (Transformation|GetActorLocation) (Math|Vector|RotateVector _leftgunloc _returnvalue)) _returnvalue (Variables|Default|GetEnergyBallScale)) false)
    (Audio|PlaySoundatLocation 0 _leftgunloc)))

(event Input|ActionEvents|InputActionFire
  (bind _returnvalue (Transformation|GetActorRotation))
  (bind _rightgunloc (Variables|Default|GetRightGunLoc))
  ;[1 1 1] Fire Guns
  (:Pressed
    (Game|SpawnActorfromClass "/Game/Blueprints/Projectile.Projectile_C" (Math|Transform|MakeTransform (+ (Transformation|GetActorLocation) (Math|Vector|RotateVector _rightgunloc _returnvalue)) _returnvalue (Variables|Default|GetEnergyBallScale)) false)
    (Audio|PlaySoundatLocation 0 _rightgunloc)))

(event Input|AxisEvents|InputAxisPitch
  (params (AxisValue :type Float%20%28single-precision%29))
  ;[1 1 1] Apply Pitch
  (Transformation|AddActorLocalRotation (Class|KismetMathLibrary|MakeRot AxisValue 0.0 0.0) false))

(event Input|AxisEvents|InputAxisRoll
  (params (AxisValue :type Float%20%28single-precision%29))
  ;[1 1 1] Apply Rotation
  (Transformation|AddActorLocalRotation (Class|KismetMathLibrary|MakeRot 0.0 (* AxisValue 0.13) 0.0) false))

(event Input|AxisEvents|InputAxisPitch
  (params (AxisValue :type Float%20%28single-precision%29))
  ;[1 1 1] Apply Pitch
  (Class|PrimitiveComponent|SetAllPhysicsLinearVelocity (Variables|Default|GetBodyMesh) (* (Math|Vector|GetForwardVector (Transformation|GetActorRotation)) (* AxisValue -0.5)) true))

(event Input|AxisEvents|InputAxisPitch
  (params (AxisValue :type Float%20%28single-precision%29))
  ;[1 1 1] Apply Pitch
  (Class|PrimitiveComponent|SetPhysicsAngularVelocity (Variables|Default|GetBodyMesh) (* (Math|Vector|GetRightVector (Transformation|GetActorRotation)) (* AxisValue -1.0)) true "None"))

(event Input|AxisEvents|InputAxisRoll
  (params (AxisValue :type Float%20%28single-precision%29))
  ;[1 1 1] Apply Rotation
  (Class|PrimitiveComponent|SetPhysicsAngularVelocity (Variables|Default|GetBodyMesh) (* (Math|Vector|GetForwardVector (Transformation|GetActorRotation)) (* AxisValue -1.0)) true "None"))

(event Input|AxisEvents|InputAxisThrust
  (params (AxisValue :type Float%20%28single-precision%29))
  ;[1 1 1] Apply foward thrust
  (Physics|SetPhysicsLinearVelocity (Variables|Default|GetBodyMesh) (* (Math|Vector|GetForwardVector (Transformation|GetActorRotation)) (* AxisValue 38.0)) true "None"))

(event Input|AxisEvents|InputAxisRoll
  (params (AxisValue :type Float%20%28single-precision%29))
  ;[1 1 1] Apply Rotation
  (Transformation|AddActorLocalRotation (Class|KismetMathLibrary|MakeRot 0.0 0.0 AxisValue) false))

(fn ConstructionScript)